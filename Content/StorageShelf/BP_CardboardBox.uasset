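; BP_CardboardBox is a cardboard box actor with two flaps that animate open and closed.
; OpenCloseBox plays or reverses a Timeline based on IsOpen, lerping the pitch of the left and right flaps in opposite directions and toggling IsOpen on finish.
; The Construction Script fills Items with two shelf slot items, whose count prints on BeginPlay as debug output.
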(event EventBeginPlay
  (Development|PrintString (Utilities|String|ToString(Integer) (Utilities|Array|Length (Variables|Default|GetItems)))))

(event EventOpenCloseBox
  (Development|PrintString "Hello")
  (if (Variables|Default|GetIsOpen)
    (bind _newtrack_0 (Timeline|Timeline Reverse)
      (:Update
        (Transformation|SetRelativeRotation (Variables|Default|GetCardboardBox_Left) (Math|Rotator|MakeRotator 0.0 (Math|Float|Lerp 45.0 -1.8e+02 _newtrack_0) 0.0) false false)
        (Transformation|SetRelativeRotation (Variables|Default|GetCardboardBox_Right) (Math|Rotator|MakeRotator 0.0 (Math|Float|Lerp -45.0 1.8e+02 _newtrack_0) 0.0) false false))
      (:Finished
        (Variables|Default|SetIsOpen (not (Variables|Default|GetIsOpen)))))
    (else
      (Timeline|Timeline Play))))

(fn ConstructionScript
  (Variables|Default|SetItems (Utilities|Array|MakeArray (Variables|Default|GetShelfSlotItem) (Variables|Default|GetShelfSlotItem1))))