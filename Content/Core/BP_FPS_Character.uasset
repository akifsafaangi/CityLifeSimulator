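; First-person player character that detects pickupable objects and shelf sections under the camera and drives the main HUD.
; BeginPlay builds the main UI, number keys switch inventory slots, and a progress event feeds the progress bar.
; A short camera line trace each tick stores the hit object and component, using a component tag to spot shelves.
; Outside placement and holding, it toggles pickup and open-box prompts and highlights targets through custom depth.
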(event EventBeginPlay
  (bind _returnvalue (UserInterface|CreateWidget "/Game/Widgets/WBP_MainUI.WBP_MainUI_C" (Game|GetPlayerController 0)))
  (bind _output_get (Variables|Default|SetMainUI _returnvalue))
  (Widget|SetVisibility (Variables|/Game/Widgets/WBP_MainUI.WBP_MainUI_C|GetWBP_Pickup_UI _output_get) "Hidden")
  (Widget|SetVisibility (Variables|/Game/Widgets/WBP_MainUI.WBP_MainUI_C|GetWBP_OpenBoxUI _output_get) "Hidden")
  (Widget|SetVisibility (Variables|/Game/Widgets/WBP_MainUI.WBP_MainUI_C|GetWBP_PlaceUI _output_get) "Hidden")
  (Variables|Default|SetInventoryHUD (Variables|/Game/Widgets/WBP_MainUI.WBP_MainUI_C|GetWBP_InventoryHUD_0 (Variables|Default|GetMainUI)))
  (UserInterface|Viewport|AddtoViewport (Variables|Default|GetMainUI) 0))

(event Collision|EventActorBeginOverlap
  (params (OtherActor :type Actor%20Object%20Reference)))

(event EventTick
  (params (DeltaSeconds :type Float%20%28single-precision%29))
  (CallFunction|LineTrace))

(event EventProgressBarPercent
  (params (percent :type Float%20%28single-precision%29))
  (Default|SetPercent (Variables|/Game/Widgets/WBP_MainUI.WBP_MainUI_C|GetWBP_ProgressBar (Variables|Default|GetMainUI)) percent))

(event Input|KeyboardEvents|1
  (params (Key :type Key%20Structure :default "None"))
  (:Pressed
    (Default|ChangeInventoryIndex (Variables|Default|GetInventoryHUD))))

(event Input|KeyboardEvents|2
  (params (Key :type Key%20Structure :default "None"))
  (:Pressed
    (Default|ChangeInventoryIndex (Variables|Default|GetInventoryHUD) 1)))

(event Input|KeyboardEvents|3
  (params (Key :type Key%20Structure :default "None"))
  (:Pressed
    (Default|ChangeInventoryIndex (Variables|Default|GetInventoryHUD) 2)))

(event Input|KeyboardEvents|4
  (params (Key :type Key%20Structure :default "None"))
  (:Pressed
    (Default|ChangeInventoryIndex (Variables|Default|GetInventoryHUD) 3)))

(event Input|KeyboardEvents|5
  (params (Key :type Key%20Structure :default "None"))
  (:Pressed
    (Default|ChangeInventoryIndex (Variables|Default|GetInventoryHUD) 4)))

(fn ConstructionScript)

(fn LineTrace
  (bind _camera (Variables|Default|GetCamera))
  (bind _returnvalue (Transformation|GetWorldLocation _camera))
  (bind (_outhit _returnvalue_2) (Collision|LineTraceByChannel _returnvalue (+ _returnvalue (* (Math|Vector|GetForwardVector (Transformation|GetWorldRotation _camera)) 5e+02)) "TraceTypeQuery3" false 0 "None"))
  (if _returnvalue_2
    (if (Components|ComponentHasTag (.HitComponent (Collision|BreakHitResult _outhit)) "ShelfSection")
      (Variables|Default|SetHitComponent (.HitComponent (Collision|BreakHitResult _outhit)))
      (bind _aspickupable_object (Utilities|Casting|CastToPickupableObject (.HitActor (Collision|BreakHitResult _outhit))))
      (Variables|Default|SetHitObject _aspickupable_object)
      (elif (not (Variables|Default|GetbIsInPlacementMode))
        (if (Variables|Default|GetbIsHolding)
          (CallFunction|ChangeBoxVisibility false)
          (CallFunction|ChangePlaceableVisibility false)
          (CallFunction|ChangePickupVisibility false)
          (else
            (bind _aspickupable_object_2 (Utilities|Casting|CastToPickupableObject (.HitActor (Collision|BreakHitResult _outhit))))
            (CallFunction|ChangePickupVisibility true)
            (Rendering|SetRenderCustomDepth (Variables|/Script/CityLifeSimulator.PickupableObject|GetStaticMesh _aspickupable_object_2) true)
            (Variables|Default|SetHitObject _aspickupable_object_2)
            (Variables|Default|SetHitComponent (.HitComponent (Collision|BreakHitResult _outhit)))
            (Utilities|Casting|CastToPlacableObject (Variables|Default|GetHitObject)
              (:CastFailed
                (CallFunction|ChangePlaceableVisibility false)
                (CallFunction|ChangeBoxVisibility true)))))))
    (else
      (CallFunction|ChangePlaceableVisibility false)
      (CallFunction|ChangeBoxVisibility false)
      (CallFunction|ChangePickupVisibility false)
      (if (Utilities|IsValid (Variables|Default|GetHitObject))
        (Rendering|SetRenderCustomDepth (Variables|/Script/CityLifeSimulator.PickupableObject|GetStaticMesh (Variables|Default|GetHitObject)) false)
        (Variables|Default|SetHitObject 0)
        (Variables|Default|SetHitComponent 0)))))

(fn ChangeBoxVisibility
  (params (Visible :type Boolean))
  (bind _mainui (Variables|Default|GetMainUI))
  (bind _wbp_openboxui (Variables|/Game/Widgets/WBP_MainUI.WBP_MainUI_C|GetWBP_OpenBoxUI _mainui))
  (if Visible
    (Widget|SetVisibility _wbp_openboxui "HitTestInvisible")
    (else
      (Widget|SetVisibility _wbp_openboxui "Hidden"))))

(fn ChangePlaceableVisibility
  (params (Visible :type Boolean))
  (bind _mainui (Variables|Default|GetMainUI))
  (bind _wbp_placeui (Variables|/Game/Widgets/WBP_MainUI.WBP_MainUI_C|GetWBP_PlaceUI _mainui))
  (if Visible
    (Widget|SetVisibility _wbp_placeui "HitTestInvisible")
    (else
      (Widget|SetVisibility _wbp_placeui "Hidden"))))

(fn ChangePickupVisibility
  (params (Visible :type Boolean))
  (bind _mainui (Variables|Default|GetMainUI))
  (bind _wbp_pickup_ui (Variables|/Game/Widgets/WBP_MainUI.WBP_MainUI_C|GetWBP_Pickup_UI _mainui))
  (if Visible
    (Widget|SetVisibility _wbp_pickup_ui "HitTestInvisible")
    (else
      (Widget|SetVisibility _wbp_pickup_ui "Hidden"))))